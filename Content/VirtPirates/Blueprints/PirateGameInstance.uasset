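; PirateGameInstance is the game instance for VirtPirates, tracking the player's current zone and coordinating save and load of level audio and actor state.
; Enter functions, sent from level triggers, set the zone index.
; Save and load pass a save object to the skull, parrot and entrance music, with game time stored in place of speaker positions.
; Debug helpers apply B2 height fog settings and print save slot contents.
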(fn `DebugRoutine`
  (params (inpHeightFog :type "ExponentialHeightFog Object Reference"))
  (bind _component (`ExponentialHeightFog.Component` inpHeightFog))
  ;[1 1 1] Debug Routine: Is called when 'x' is pressed.
  ;[1 1 1] Set ground fog for B2
  (`ExponentialHeightFogComponent.SetFogDensity` _component 0.010366)
  (`ExponentialHeightFogComponent.SetFogInscatteringColor` _component (struct :`R` 1.0 :`G` 0.919393 :`B` 0.905 :`A` 1.0))
  (`ExponentialHeightFogComponent.SetFogHeightFalloff` _component 0.037679)
  (`ExponentialHeightFogComponent.SetFogMaxOpacity` _component 0.5)
  (`ExponentialHeightFogComponent.SetStartDistance` _component 0.0))

(fn `Enter_B1`
  (set `self.GI_nCurrentZone` 0) ; Update We are going into B1
)

(fn `Enter_B2a`
  (locals (loc_Boat0Speed :type "Float (double-precision)") (locStoredRotation :type "Rotator Structure"))
  (set `self.GI_nCurrentZone` 2) ; Update We are going into Grotto A
)

(fn `Enter_B2b`
  (set `self.GI_nCurrentZone` 3))

(fn `Enter_Ga`
  (locals (loc_Boat0Speed :type "Float (double-precision)") (loc_storedRotation :type "Rotator Structure"))
  ;[1 1 1] Sent from tripped level trigger B1G1 by way of Level BP function
  (set `self.GI_nCurrentZone` 1) ; Update We are going into Grotto A
)

(fn `Enter_Gb`
  (set `self.GI_nCurrentZone` 4))

(fn `LoadLevel1AA`
  (params (pSaveGame :type "/Game/VirtPirates/Blueprints/PirateSaveGame Object Reference"))
  ;[1 1 1] Called from LBP Event Graph
  (`/Game/VirtPirates/VP_Mesh/Building_1/Arches/TalkingSkull/AABP_Skull.LoadSkull` (`self.pAABP_Skull`) pSaveGame)
  (`/Game/VirtPirates/VP_Mesh/Building_1/2_Entrance/8_ParrotIsland/Blueprints/BP_Parrot.LoadParrot` (`self.pParrot`) pSaveGame)
  (`/Game/VirtPirates/VP_Mesh/Building_1/2_Entrance/2_EntranceWalls/Sounds/BP_EntranceMusic.LoadEnSound` (`self.pEntranceMusic`) pSaveGame))

(fn `PrintSaveFile`
  (params (in_FIleNumber :type Integer))
  (locals (pSaveFile :type "/Game/VirtPirates/Blueprints/PirateSaveGame Object Reference") (loc_String :type "Array of String") (NewLocalVar_2 :type "Float (double-precision)"))
  (bind _output (`|GetArrayItem` (`local.loc_String`) in_FIleNumber))
  (`KismetSystemLibrary.PrintString` "sf")
  (`KismetSystemLibrary.PrintString` (`KismetStringLibrary.Concat_StrStr` "sfPrint File: " (`KismetStringLibrary.Conv_IntToString` in_FIleNumber)))
  (bind _returnvalue (`GameplayStatics.DoesSaveGameExist` _output)) ; Does requested file exist?
  (if _returnvalue
    (bind _returnvalue_2 (`GameplayStatics.LoadGameFromSlot` _output))
    (bind _aspirate_save_game (cast `/Game/VirtPirates/Blueprints/PirateSaveGame` _returnvalue_2))
    (bind _output_get (set `local.pSaveFile` _aspirate_save_game))
    (`KismetSystemLibrary.PrintString` (`KismetStringLibrary.Concat_StrStr` "sfSkull Playing: " (`KismetStringLibrary.Conv_BoolToString` (`/Game/VirtPirates/Blueprints/PirateSaveGame.bSkullPlaying` _output_get))))
    (`KismetSystemLibrary.PrintString` (`KismetStringLibrary.Concat_StrStr` "sfPlay Position: " (`KismetStringLibrary.Conv_DoubleToString` (`/Game/VirtPirates/Blueprints/PirateSaveGame.SkullPlayPosition` _output_get))))
    (`KismetSystemLibrary.PrintString` (`KismetStringLibrary.Concat_StrStr` "sfCurrentZone: " (`KismetStringLibrary.Conv_IntToString` (`/Game/VirtPirates/Blueprints/PirateSaveGame.nCurrentZone` _output_get))))
    (`KismetSystemLibrary.PrintString` (`KismetStringLibrary.Concat_StrStr` "sfIn Boat: " (`KismetStringLibrary.Conv_BoolToString` (`/Game/VirtPirates/Blueprints/PirateSaveGame.bInBoat` _output_get))))
    (`KismetSystemLibrary.PrintString` (`KismetStringLibrary.Concat_StrStr` "sfBoat Index: " (`KismetStringLibrary.Conv_IntToString` (`/Game/VirtPirates/Blueprints/PirateSaveGame.nBoatIndex` _output_get))))
    (else
      (`KismetSystemLibrary.PrintString` (`KismetStringLibrary.Concat_StrStr` _output " Doesn't Exist.")))))

(fn `SaveLevel1AA`
  (params (pSaveFile :type "/Game/VirtPirates/Blueprints/PirateSaveGame Object Reference"))
  ;[1 1 1] No easy way to get current positiion of speakers, so I'll use game time.
  (set `/Game/VirtPirates/Blueprints/PirateSaveGame.GameTime` (`KismetSystemLibrary.GetGameTimeInSeconds`) pSaveFile)
  (`/Game/VirtPirates/VP_Mesh/Building_1/Arches/TalkingSkull/AABP_Skull.SaveSkull` (`self.pAABP_Skull`) pSaveFile)
  (`/Game/VirtPirates/VP_Mesh/Building_1/2_Entrance/8_ParrotIsland/Blueprints/BP_Parrot.SaveParrot` (`self.pParrot`) pSaveFile)
  (`/Game/VirtPirates/VP_Mesh/Building_1/2_Entrance/2_EntranceWalls/Sounds/BP_EntranceMusic.SaveEnSound` (`self.pEntranceMusic`) pSaveFile))