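; Level transition trigger between zones Gb and B1 in VirtPirates, working in both directions.
; On overlap it accepts only the player pawn, ignoring other actors such as the boat, then reads the current zone from PirateGameInstance.
; That zone selects whether it calls the Gb-to-B1 or B1-to-Gb level change; any other zone does nothing.
; The level change itself is handled outside this graph.
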(event `self.ReceiveActorBeginOverlap`
  (params (OtherActor :type "Actor Object Reference"))
  ;[1 1 1] Verify that other actor is Player, not boat
  (if (== OtherActor (`GameplayStatics.GetPlayerPawn` 0))
    ;[1 1 1] Check zone
    (bind _aspirate_game_instance (cast `/Game/VirtPirates/Blueprints/PirateGameInstance` (`GameplayStatics.GetGameInstance`)))
    (bind _gi_ncurrentzone (`/Game/VirtPirates/Blueprints/PirateGameInstance.GI_nCurrentZone` _aspirate_game_instance))
    (if (== _gi_ncurrentzone 4)
      (`self.LevelChange_GbB1`)
      (elif (== _gi_ncurrentzone 0)
        (`self.LevelChange_B1Gb`)))))

(fn `UserConstructionScript`)