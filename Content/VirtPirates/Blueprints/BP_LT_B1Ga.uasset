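; BP_LT_B1Ga is a level transition trigger between the B1 and Ga areas.
; On overlap it ignores any actor other than player 0's pawn, such as the boat, then reads GINCurrentZone from PirateGameInstance.
; Zone 0 calls LevelChangeB1Ga and zone 1 calls LevelChangeGaB1, so one trigger serves both directions.
; The level change itself is handled outside this graph, and other zones or a failed cast only print debug text.
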(event `self.ReceiveActorBeginOverlap`
  (params (OtherActor :type "Actor Object Reference"))
  ;[1 1 1] Verify that other actor is Player, not boat
  (if (== OtherActor (`GameplayStatics.GetPlayerPawn` 0))
    ;[1 1 1] Get current zone number...
    (bind _aspirate_game_instance (cast `/Game/VirtPirates/Blueprints/PirateGameInstance` (`GameplayStatics.GetGameInstance`))
      (:`then`
        (bind _gi_ncurrentzone (`/Game/VirtPirates/Blueprints/PirateGameInstance.GI_nCurrentZone` _aspirate_game_instance))
        (if (== _gi_ncurrentzone 0)
          (`self.LevelChange_B1Ga`)
          (elif (== _gi_ncurrentzone 1)
            (`self.LevelChange_GaB1`)
            (else
              (`KismetSystemLibrary.PrintText` "Bad Switch")))))
      (:`CastFailed`
        (`KismetSystemLibrary.PrintText` "Cast Failed")))))

(fn `UserConstructionScript`)