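; BP_LT_B2aB2b is a level-transition trigger between zones B2a and B2b in VirtPirates.
; On overlap by the player pawn, it reads the current zone number from PirateGameInstance, ignoring other actors such as an empty boat.
; That number selects the direction, calling the matching B2a-to-B2b or B2b-to-B2a level change, or printing an error for any other zone.
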(event `self.ReceiveActorBeginOverlap`
  (params (OtherActor :type "Actor Object Reference"))
  ;[1 1 1] Verify that other actor is Player, not empty boat
  (if (== OtherActor (`GameplayStatics.GetPlayerPawn` 0))
    ;[1 1 1] Check zone
    (bind _aspirate_game_instance (cast `/Game/VirtPirates/Blueprints/PirateGameInstance` (`GameplayStatics.GetGameInstance`)))
    (bind _gi_ncurrentzone (`/Game/VirtPirates/Blueprints/PirateGameInstance.GI_nCurrentZone` _aspirate_game_instance))
    (if (== _gi_ncurrentzone 2)
      (`self.LevelChange_B2aB2b`)
      (elif (== _gi_ncurrentzone 3)
        (`self.LevelChange_B2bB2a`)
        (else
          (`KismetSystemLibrary.PrintString` "Bad zone No"))))))

(fn `UserConstructionScript`)