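; BP_Cannon is a cannon actor that plays animation, sound and visual effects when its fire event is triggered.
; Firing starts a timeline that colors and animates the muzzle spew's dynamic material, tints a point light and activates a particle system.
; Each tick pitches the flat spew rectangle toward the camera and fades it by relative yaw, hiding it when viewed straight on.
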(event `self.ReceiveBeginPlay`
  (`self.EnableInput` (`GameplayStatics.GetPlayerController` 0))
  (add `self.FireEvent` (delegate `FireEvent_Event`)))

(event `FireEvent_Event`
  (`SkeletalMeshComponent.PlayAnimation` (`self.SkeletalMesh`) "/Game/VirtPirates/VP_Mesh/Building_2/Fort/ShipCannon/Cannon/AnimCannon_Anim.AnimCannon_Anim" false) ; Imported Cannon Animation
  (`AudioComponent.Play` (`self.Depth_Charge_Short-SoundBible_com-1303947570_Cue`) 0.0)
  (bind (_direction _ialightcolor _spewcolor) (`Timeline|Timeline_1` :!via `PlayFromStart`)
    (:`Update`
      (`MaterialInstanceDynamic.SetVectorParameterValue` (`self.SpewRectMatl`) "Colorize" _spewcolor) ; Color the spew
      (`MaterialInstanceDynamic.SetScalarParameterValue` (`self.SpewRectMatl`) "CurrentTime" (`TimelineComponent.GetPlaybackPosition` (`self.Timeline_1`))) ; Animate the material
      (`LightComponent.SetLightColor` (`self.PointLight`) _ialightcolor true) ; Set the IA Light color
    )
    (:`Finished`
      (`TimelineComponent.Stop` (`self.Timeline_1`)))
    (:`Event`
      (`ActorComponent.Activate` (`self.ParticleSystem`) true))))

(event `self.ReceiveActorBeginOverlap`
  (params (OtherActor :type "Actor Object Reference")))

(event `self.ReceiveTick`
  (params (DeltaSeconds :type "Float (single-precision)"))
  (bind _skeletalmesh (`self.SkeletalMesh`))
  (bind _spewrect (`self.SpewRect`))
  (`SceneComponent.K2_SetWorldRotation` (`self.SpewRect`) (`KismetMathLibrary.MakeRotator` (.roll (`SceneComponent.K2_GetComponentRotation` _spewrect)) (.pitch (`KismetMathLibrary.FindLookAtRotation` (`SceneComponent.K2_GetComponentLocation` _spewrect) (`PlayerCameraManager.GetCameraLocation` (`PlayerController.PlayerCameraManager` (`GameplayStatics.GetPlayerController` 0))))) (.yaw (`SceneComponent.K2_GetComponentRotation` _spewrect))) false false) ; Rotate towards Camera in Y
  (`MaterialInstanceDynamic.SetScalarParameterValue` (`self.SpewRectMatl`) "Opacity" (`KismetMathLibrary.FClamp` (- (`KismetMathLibrary.Abs` (* (- (- (.yaw (`SceneComponent.K2_GetComponentRotation` _skeletalmesh)) (.yaw (`KismetMathLibrary.FindLookAtRotation` (`PlayerCameraManager.GetCameraLocation` (`PlayerController.PlayerCameraManager` (`GameplayStatics.GetPlayerController` 0))) (`SceneComponent.K2_GetComponentLocation` _skeletalmesh)))) 90.0) 0.025)) 0.5))) ; Spew fades if we start to look straight on
)

(fn `AngleBetweenVectors`
  (params (V1 :type "Vector Structure") (V2 :type "Vector Structure"))
  (returns (outAngle :type "Float (double-precision)"))
  (return (`KismetMathLibrary.DegAcos` (`KismetMathLibrary.Dot_VectorVector` (`KismetMathLibrary.Normal` V1) (`KismetMathLibrary.Normal` V2)))))

(fn `UserConstructionScript`
  (bind _returnvalue (`PrimitiveComponent.CreateDynamicMaterialInstance` (`self.SpewRect`) 0 null))
  (set `self.SpewRectMatl` _returnvalue))