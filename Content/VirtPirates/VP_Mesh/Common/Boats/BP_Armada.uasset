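; BP_Armada manages a fleet of boat locators that travel along splines.
; InitGameArmada, called from the Level Blueprint, sizes the fleet to ArmadaSize, resets each boat, and assigns its spline, distance and speed from data table rows.
; Fleet-wide functions pause, destroy, save, load and toggle collision by looping over the locators, with input bindings for pause and collision.
; Getters expose boats, splines, defaults and the wrap-around index of the boat ahead.
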(event `self.ReceiveBeginPlay`)

(event `Key|Backslash`
  (params (Key :type "Key Structure"))
  (:`Released`
    (`self.ToggleCollision` (not (`self.bCollisionEnabled`)))))

(event `InputAction|PauseBoats`
  (params (Key :type "Key Structure"))
  (:`Pressed`
    (`self.TogglePauseArmada`)))

(event `InputAction|EnterBoatZero`
  (params (Key :type "Key Structure")))

(fn `CM_to_Feet`
  (params (in_CM :type "Float (double-precision)"))
  (returns (ret_Feet :type "Float (double-precision)"))
  (return (/ in_CM 30.48)))

(fn `GetBoatLocation`
  (params (inIndex :type Integer))
  (returns (outLocation :type "Float (double-precision)"))
  ;[1 1 1] Currently not called.
  (bind _retboatprogress (`/Game/VirtPirates/VP_Mesh/Common/Boats/BP_Boat_Locator.GetBoatSplinePosition` (`|GetArrayItem` (`self.aLocators`) inIndex)))
  (return _retboatprogress))

(fn `GetDefBoatSpeed`
  (returns (retBoatSpeed :type "Float (double-precision)"))
  (return (`self.DefBoatSpeed`)))

(fn `GetDefBobRate`
  (returns (RetBobRate :type "Float (double-precision)"))
  (return (`self.DefBobRate`)))

(fn `GetpBoat`
  (params (inBoatIndex :type Integer))
  (returns (retpBoat :type "/Game/VirtPirates/VP_Mesh/Common/Boats/BP_Boat_Locator Object Reference"))
  (if (> inBoatIndex 5)
    (`KismetSystemLibrary.PrintString` "Boat Index Out of Range")
    (else
      (return (`|GetArrayItem` (`self.aLocators`) inBoatIndex)))))

(fn `GetpSplineByIndex`
  (params (in_SplineIndex :type Integer))
  (returns (out_pSpline :type "/Game/VirtPirates/VP_Mesh/Common/Boats/BP_BoatSpline Object Reference"))
  (return (`|GetArrayItem` (`self.aBoatSplines`) in_SplineIndex)))

(fn `GetUpstreamBoatIndex`
  (params (in_nCallingBoatIndex :type Integer))
  (returns (retUSInt :type Integer))
  (locals (loc_testIndex :type Integer) (loc_returnIndex :type Integer))
  (return (mod (+ in_nCallingBoatIndex 1) (`self.ArmadaSize`))))

(fn `Init_Game_Armada`
  (params (ArrayOfBoatLocators :type "Array of /Game/VirtPirates/VP_Mesh/Common/Boats/BP_Boat_Locator Object Reference"))
  (locals (loc_pCurrentBoat :type "/Game/VirtPirates/VP_Mesh/Common/Boats/BP_Boat_Locator Object Reference") (loc_aBoatNames :type "Array of Name") (loc_BoatIndex :type Integer) (loc_SplineIndex :type Integer) (loc_StartingDistance :type "Float (double-precision)") (loc_startingSpeed :type "Float (double-precision)") (loc_StartBobRate :type "Float (double-precision)"))
  ;[1 1 1] Called from Level Blueprint: EventBeginPlay
  (`|ExecutionSequence`
    (:`then_0`
      (set `self.aLocators` ArrayOfBoatLocators) ; Init our variable
    )
    (:`then_1`
      (if (not (== (`self.ArmadaSize`) (`KismetArrayLibrary.Array_Length` (`self.aLocators`))))
        ;[1 1 1] Allow Armada size < 20
        (`KismetArrayLibrary.Array_Resize` (`self.aLocators`) (`self.ArmadaSize`)))
      ;[1 1 1] For Each Boat Locator
      (for (_array_element _array_index) (`self.aLocators`)
        (`|ExecutionSequence`
          (:`then_0`
            (set `local.loc_pCurrentBoat` _array_element) ; store local copy
            (set `local.loc_BoatIndex` _array_index))
          (:`then_1`
            (`/Game/VirtPirates/VP_Mesh/Common/Boats/BP_Boat_Locator.ResetBoat` (`local.loc_pCurrentBoat`) (`local.loc_BoatIndex`)))
          (:`then_2`
            (bind _returnvalue (`|GetDataTableRow` "/Game/VirtPirates/VP_Mesh/Common/Boats/ArmadaData.ArmadaData" (`|GetArrayItem` (`local.loc_aBoatNames`) (`local.loc_BoatIndex`)))
              (:`then`
                (bind (_spline _distance _speedfactor _bobrate) (break `/Game/VirtPirates/VP_Mesh/Common/Boats/ArmadaSturcture` _returnvalue))
                ;[1 1 1] Set local variables from .csv file
                (set `local.loc_SplineIndex` _spline)
                (set `local.loc_StartingDistance` _distance)
                (set `local.loc_startingSpeed` _speedfactor)
                (set `local.loc_StartBobRate` _bobrate))))
          (:`then_3`
            (`/Game/VirtPirates/VP_Mesh/Common/Boats/BP_Boat_Locator.SetLocatorSpline` (`local.loc_pCurrentBoat`) (`|GetArrayItem` (`self.aBoatSplines`) (`local.loc_SplineIndex`)) 0) ; Call BPBoatLocator::SetLocatorSpline
          )
          (:`then_4`
            (`/Game/VirtPirates/VP_Mesh/Common/Boats/BP_Boat_Locator.SetBoatProgress` (`local.loc_pCurrentBoat`) (`local.loc_StartingDistance`))
            (`/Game/VirtPirates/VP_Mesh/Common/Boats/BP_Boat_Locator.SetBoatSpeed` (`local.loc_pCurrentBoat`) (* (`self.DefBoatSpeed`) (`local.loc_startingSpeed`))))
          (:`then_5`
            (set `/Game/VirtPirates/VP_Mesh/Common/Boats/BP_Boat_Locator.bIsPaused` false (`local.loc_pCurrentBoat`)) ; Un-pause boat
          )
          (:`then_6`
            (bind _asboat_abp (cast `/Game/VirtPirates/VP_Mesh/Common/Boats/Boat_Animations/Boat_ABP` (`SkeletalMeshComponent.GetAnimInstance` (`/Game/VirtPirates/VP_Mesh/Common/Boats/BP_Boat_Locator.Boat_SM` (`local.loc_pCurrentBoat`))))
              (:`then`
                (`/Game/VirtPirates/VP_Mesh/Common/Boats/Boat_Animations/Boat_ABP.SetBobRate` _asboat_abp 0.0))
              (:`CastFailed`
                (`KismetSystemLibrary.PrintString` "Cast Failed in BobRate")))))))))

(fn `KillBoats`
  ;[1 1 1] For Each Boat Locator
  (for _array_element (`self.aLocators`)
    (`self.K2_DestroyActor` _array_element)))

(fn `LoadArmadaData`
  (params (in_pSaveFile :type "/Game/VirtPirates/Blueprints/PirateSaveGame Object Reference"))
  (locals (locpLocator :type "/Game/VirtPirates/VP_Mesh/Common/Boats/BP_Boat_Locator Object Reference") (locpSaveFile :type "/Game/VirtPirates/Blueprints/PirateSaveGame Object Reference") (locDataIndex :type Integer) (loc_CurrentZone :type Integer))
  (set `local.locpSaveFile` in_pSaveFile)
  ;[1 1 1] For Each Boat Locator
  (for _array_element (`self.aLocators`)
    (`/Game/VirtPirates/VP_Mesh/Common/Boats/BP_Boat_Locator.LoadBoat` _array_element (`local.locpSaveFile`) (`self.aBoatSplines`)))
  (return))

(fn `SaveArmadaData`
  (params (pSaveFile :type "/Game/VirtPirates/Blueprints/PirateSaveGame Object Reference"))
  (locals (locpSaveFile :type "/Game/VirtPirates/Blueprints/PirateSaveGame Object Reference"))
  (set `local.locpSaveFile` pSaveFile) ; Save local
  ;[1 1 1] For Each Boat Locator
  (for _array_element (`self.aLocators`)
    ;[1 1 1] Save Each Boat Locator
    (`/Game/VirtPirates/VP_Mesh/Common/Boats/BP_Boat_Locator.SaveBoat` _array_element (`local.locpSaveFile`))))

(fn `ToggleCollision`
  (params (in_bwantCollision :type Boolean))
  (locals (enumColType :type "ECollisionEnabled Enum"))
  (if in_bwantCollision
    (set `local.enumColType` "PhysicsOnly")
    (else
      (set `local.enumColType` "NoCollision")))
  (for _array_element (`self.aLocators`)
    (`PrimitiveComponent.SetCollisionEnabled` (`/Game/VirtPirates/VP_Mesh/Common/Boats/BP_Boat_Locator.Boat_SM` _array_element) (`local.enumColType`))))

(fn `TogglePauseArmada`
  ;[1 1 1] For Each Boat Locator
  (for _array_element (`self.aLocators`)
    ;[1 1 1] Call Toggle Pause on the boat
    (`/Game/VirtPirates/VP_Mesh/Common/Boats/BP_Boat_Locator.TogglePause` _array_element)))

(fn `UserConstructionScript`)