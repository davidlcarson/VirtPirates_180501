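; A boat trigger actor that temporarily pauses the boat that trips it.
; On overlap it runs the parent handler, then, if a tripping boat is set, ramps that boat's speed increment down to zero.
; After the ramp-down time plus a pause duration, it ramps the boat back up to the armada's default speed scaled by a resume factor.
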(event `self.ReceiveActorBeginOverlap`
  (params (OtherActor :type "Actor Object Reference"))
  (`parent.ReceiveActorBeginOverlap` OtherActor)
  (if (not (== (`self.pTrippingBoat`) null))
    (`|ExecutionSequence`
      (:`then_0`
        (`/Game/VirtPirates/VP_Mesh/Common/Boats/BP_Boat_Locator.RampToIncrement` (`self.pTrippingBoat`) 0.0 (`self.RampDownTime`)) ; Ramp down to 0
      )
      (:`then_1`
        (`KismetSystemLibrary.Delay` (+ (`self.RampDownTime`) (`self.PauseDuration`)))
        (bind _retboatspeed (`/Game/VirtPirates/VP_Mesh/Common/Boats/BP_Armada.GetDefBoatSpeed` (`self.pArmada`)))
        (`/Game/VirtPirates/VP_Mesh/Common/Boats/BP_Boat_Locator.RampToIncrement` (`self.pTrippingBoat`) (* _retboatspeed (`self.ResumeFactor`)) (`self.ResumeTime`)))
      (:`then_2`))))

(fn `UserConstructionScript`
  (`parent.UserConstructionScript`))