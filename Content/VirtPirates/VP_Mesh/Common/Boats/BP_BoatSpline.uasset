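; BP_BoatSpline is a spline path actor for boats, exposing an ID and a length through getter functions.
; It caches the spline length on BeginPlay and resets progress to zero on any BP_Boat_Locator that begins overlapping the spline component.
; The construction script only reads the point count, as its loop for flattening points to a desired height is disconnected.
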(event `self.ReceiveBeginPlay`
  (set `self.m_SplineLength` (`SplineComponent.GetSplineLength` (`self.BoatSpline`))))

(event `self.BoatSpline.OnComponentBeginOverlap`
  (params (OverlappedComponent :type "PrimitiveComponent Object Reference") (OtherActor :type "Actor Object Reference") (OtherComp :type "PrimitiveComponent Object Reference") (OtherBodyIndex :type Integer) (bFromSweep :type Boolean) (SweepResult :type "HitResult Structure (by ref)"))
  (bind _asbp_boat_locator (cast `/Game/VirtPirates/VP_Mesh/Common/Boats/BP_Boat_Locator` OtherActor))
  (`/Game/VirtPirates/VP_Mesh/Common/Boats/BP_Boat_Locator.SetBoatProgress` _asbp_boat_locator 0.0))

(fn `GetID`
  (returns (ret_nID :type Integer))
  (return (`self.splineID`)))

(fn `GetSplineLength`
  (returns (retSplineLength :type "Float (double-precision)"))
  (return (`self.m_SplineLength`)))

(fn `UserConstructionScript`
  (locals (loc_Vector :type "Vector Structure"))
  (set `self.NumberPoints` (`SplineComponent.GetNumberOfSplinePoints` (`self.BoatSpline`))))