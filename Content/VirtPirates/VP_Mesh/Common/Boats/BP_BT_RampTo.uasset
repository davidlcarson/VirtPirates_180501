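; Trigger actor that ramps a boat's speed to a fraction or multiple of the default boat speed.
; On overlap it runs the parent's handler, then checks that the tripping boat reference is set.
; It scales the armada's default boat speed by SpeedFactor and passes that to the boat's RampToIncrement along with RampTime.
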(event `self.ReceiveActorBeginOverlap`
  (params (OtherActor :type "Actor Object Reference"))
  (`parent.ReceiveActorBeginOverlap` OtherActor)
  (if (not (== (`self.pTrippingBoat`) null))
    ;[1 1 1] Ramp a boat to a factor of the default boat speed
    (bind _retboatspeed (`/Game/VirtPirates/VP_Mesh/Common/Boats/BP_Armada.GetDefBoatSpeed` (`self.pArmada`)))
    (`/Game/VirtPirates/VP_Mesh/Common/Boats/BP_Boat_Locator.RampToIncrement` (`self.pTrippingBoat`) (* _retboatspeed (`self.SpeedFactor`)) (`self.RampTime`))))

(event `self.ReceiveTick`
  (params (DeltaSeconds :type "Float (single-precision)"))
  (`parent.ReceiveTick` DeltaSeconds))

(fn `UserConstructionScript`
  (`parent.UserConstructionScript`))