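; BP_BT_EndOfSpline is an overlap trigger that moves a boat onto another spline, presumably where its current one ends.
; On overlap it acts on its referenced tripping boat, skipping it if already on the target spline index.
; It gets the target spline from the armada by index, assigns it to the boat, then sets the new progress distance, leaving speed and acceleration unchanged.
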(event `self.ReceiveActorBeginOverlap`
  (params (OtherActor :type "Actor Object Reference"))
  (`parent.ReceiveActorBeginOverlap` OtherActor)
  (if (== (`self.pTrippingBoat`) null)
    _
    (elif (not (== (`self.ndxNextSpline`) (`/Game/VirtPirates/VP_Mesh/Common/Boats/BP_Boat_Locator.nSplineIndex` (`self.pTrippingBoat`))))
      (`|ExecutionSequence`
        (:`then_0`
          (bind _out_pspline (`/Game/VirtPirates/VP_Mesh/Common/Boats/BP_Armada.GetpSplineByIndex` (`self.pArmada`) (`self.ndxNextSpline`))))
        (:`then_1`
          (`/Game/VirtPirates/VP_Mesh/Common/Boats/BP_Boat_Locator.SetLocatorSpline` (`self.pTrippingBoat`) _out_pspline (`self.ndxNextSpline`)))
        (:`then_2`
          (`/Game/VirtPirates/VP_Mesh/Common/Boats/BP_Boat_Locator.SetBoatProgress` (`self.pTrippingBoat`) (`self.newDistance`)) ; speed, accel unchanged
        )))))

(fn `UserConstructionScript`
  (`parent.UserConstructionScript`))