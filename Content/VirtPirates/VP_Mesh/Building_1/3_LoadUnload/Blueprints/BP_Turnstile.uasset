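; Turnstile gate actor with left and right flaps that swing open on request and close by themselves after a short delay.
; OpenGate calls OpenGatesEvent, which ignores requests while GateOpen is set and otherwise plays a timeline pitching the flaps in opposite directions.
; When the timeline finishes opening, it waits, clears GateOpen and reverses from the end, with the flag check preventing a loop.
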(event `self.ReceiveBeginPlay`)

(event `OpenGatesEvent`
  (bind _leftflap (`self.LeftFlap`))
  (bind _rightflap (`self.RightFlap`))
  (if (not (`self.bGateOpen`))
    (set `self.bGateOpen` true)
    (bind (_direction _flaprotation) (`Timeline|Timeline_0` :!label _label)
      (:`Update`
        (`SceneComponent.K2_SetRelativeRotation` _rightflap (`KismetMathLibrary.MakeRotator` (.roll (`SceneComponent.RelativeRotation` _rightflap)) (* _flaprotation -1.0) (.yaw (`SceneComponent.RelativeRotation` _rightflap))) false false)
        (`SceneComponent.K2_SetRelativeRotation` _leftflap (`KismetMathLibrary.MakeRotator` (.roll (`SceneComponent.RelativeRotation` _leftflap)) _flaprotation (.yaw (`SceneComponent.RelativeRotation` _leftflap))) false false))
      (:`Finished`
        (if (`self.bGateOpen`)
          (`KismetSystemLibrary.Delay` 3.5)
          (set `self.bGateOpen` false)
          (goto _label :!via `ReverseFromEnd`))))))

(fn `OpenGate`
  (`self.OpenGatesEvent`))

(fn `UserConstructionScript`)