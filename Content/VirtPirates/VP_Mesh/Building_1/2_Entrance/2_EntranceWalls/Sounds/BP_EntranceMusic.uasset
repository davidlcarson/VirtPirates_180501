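; BP_EntranceMusic plays the entrance music through four speaker components that start and stop together.
; Activate and deactivate functions are guarded by IsPlaying; a zero start time is replaced by game time modulo SoundDuration.
; Save and load functions persist the playing state and an estimated position derived from game time rather than actual playback.
; Loading always stops the speakers, then resumes at the saved position if music was playing.
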(fn `EnSound_Activate`
  (params (StartTime :type "Float (double-precision)"))
  (locals (lStartTime :type "Float (double-precision)"))
  (bind _speaker_1 (`self.Speaker_1`))
  (bind _speaker_2 (`self.Speaker_2`))
  (bind _speaker_3 (`self.Speaker_3`))
  (bind _speaker_4 (`self.Speaker_4`))
  (bind _lstarttime (`local.lStartTime`))
  (if (not (`self.bIsPlaying`))
    (if (== StartTime 0.0)
      (set `local.lStartTime` (mod (`KismetSystemLibrary.GetGameTimeInSeconds`) (`self.SoundDuration`)))
      (else
        (set `local.lStartTime` StartTime)))
    (`ActorComponent.Activate` _speaker_1 false)
    (`AudioComponent.Play` _speaker_1 _lstarttime)
    (`ActorComponent.Activate` _speaker_2 false)
    (`AudioComponent.Play` _speaker_2 _lstarttime)
    (`ActorComponent.Activate` _speaker_3 false)
    (`AudioComponent.Play` _speaker_3 _lstarttime)
    (`ActorComponent.Activate` _speaker_4 false)
    (`AudioComponent.Play` _speaker_4 _lstarttime)
    (set `self.bIsPlaying` true)))

(fn `EnSoundDeActivate`
  (if (`self.bIsPlaying`)
    (`ActorComponent.Deactivate` (`self.Speaker_1`))
    (`ActorComponent.Deactivate` (`self.Speaker_2`))
    (`ActorComponent.Deactivate` (`self.Speaker_3`))
    (`ActorComponent.Deactivate` (`self.Speaker_4`))
    (set `self.bIsPlaying` false)))

(fn `LoadEnSound`
  (params (pPirateSave :type "/Game/VirtPirates/Blueprints/PirateSaveGame Object Reference"))
  ;[1 1 1] Called by:
  (`self.EnSoundDeActivate`) ; Always deactivate...
  (if (`/Game/VirtPirates/Blueprints/PirateSaveGame.bEnSoundPlaying` pPirateSave)
    (`self.EnSound_Activate` (`/Game/VirtPirates/Blueprints/PirateSaveGame.EnSoundPosition` pPirateSave)) ; Now activate if desired
  ))

(fn `SaveEnSound`
  (params (pPiratteSave :type "/Game/VirtPirates/Blueprints/PirateSaveGame Object Reference"))
  (locals (NewLocalVar_0 :type "Float (double-precision)"))
  ;[1 1 1] Called by:
  (bind _output_get (set `/Game/VirtPirates/Blueprints/PirateSaveGame.bEnSoundPlaying` (`self.bIsPlaying`) pPiratteSave))
  (if _output_get
    (set `/Game/VirtPirates/Blueprints/PirateSaveGame.EnSoundPosition` (mod (`KismetSystemLibrary.GetGameTimeInSeconds`) (`self.SoundDuration`)) pPiratteSave)))

(fn `UserConstructionScript`)