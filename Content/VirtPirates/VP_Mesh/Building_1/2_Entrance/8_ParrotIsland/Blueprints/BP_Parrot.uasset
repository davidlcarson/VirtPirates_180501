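; Parrot actor for the VirtPirates Parrot Island area that toggles a looping animation and its sound on and off.
; ParrotActivate plays ParrotAA and starts the sound cue at a random offset within its first 25 seconds, while ParrotDeactivate stops both.
; An IsPlaying flag is written to the pirate save, and loading reactivates or stops the parrot from it without restoring playback position.
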(fn `LoadParrot`
  (params (pPirateSave :type "/Game/VirtPirates/Blueprints/PirateSaveGame Object Reference"))
  (if (`/Game/VirtPirates/Blueprints/PirateSaveGame.bParrotPlaying` pPirateSave)
    ;[1 1 1] No sync or position
    (`self.ParrotActivate`)
    (else
      (`self.ParrotDeactivate`))))

(fn `ParrotActivate`
  (bind _parrotsoundcue (`self.ParrotSoundCue`))
  (`SkeletalMeshComponent.Play` (`self.ParrotAA`) true)
  (`ActorComponent.Activate` _parrotsoundcue false)
  (`AudioComponent.Play` _parrotsoundcue (* 25.0 (`KismetMathLibrary.RandomFloat`)))
  (set `self.bIsPlaying` true))

(fn `ParrotDeactivate`
  (`SkeletalMeshComponent.Stop` (`self.ParrotAA`))
  (`ActorComponent.Deactivate` (`self.ParrotSoundCue`))
  (set `self.bIsPlaying` false))

(fn `SaveParrot`
  (params (pPirateSave :type "/Game/VirtPirates/Blueprints/PirateSaveGame Object Reference"))
  (set `/Game/VirtPirates/Blueprints/PirateSaveGame.bParrotPlaying` (`self.bIsPlaying`) pPirateSave))

(fn `UserConstructionScript`)