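; BP_DRMusic is an actor that switches the Downramp area's music and waterfall audio on and off as the player passes through two trigger boxes.
; BoxTrigger_1 activates three speakers and a waterfall speaker, and BoxTrigger_2 deactivates them, guarded by an IsPlaying flag.
; The three speakers start at game time modulo SoundDuration, keeping playback aligned to a continuous timeline, while the waterfall starts from zero.
; The load and save functions are empty.
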(event `self.ReceiveBeginPlay`)

(event `self.BoxTrigger_1.OnComponentBeginOverlap`
  (params (OverlappedComponent :type "PrimitiveComponent Object Reference") (OtherActor :type "Actor Object Reference") (OtherComp :type "PrimitiveComponent Object Reference") (OtherBodyIndex :type Integer) (bFromSweep :type Boolean) (SweepResult :type "HitResult Structure (by ref)"))
  ;[1 1 1] make sure is player
  (if (== OtherActor (`GameplayStatics.GetPlayerPawn` 0))
    (if (not (`self.bIsPlaying`))
      (`self.Activate_DRMusic`))))

(event `self.BoxTrigger_2.OnComponentBeginOverlap`
  (params (OverlappedComponent :type "PrimitiveComponent Object Reference") (OtherActor :type "Actor Object Reference") (OtherComp :type "PrimitiveComponent Object Reference") (OtherBodyIndex :type Integer) (bFromSweep :type Boolean) (SweepResult :type "HitResult Structure (by ref)"))
  ;[1 1 1] make sure is player
  (if (== OtherActor (`GameplayStatics.GetPlayerPawn` 0))
    (if (`self.bIsPlaying`)
      (`self.Deactivate_DRMusic`))))

(fn `Activate_DRMusic`
  (bind _speaker_1 (`self.Speaker_1`))
  (bind _speaker_2 (`self.Speaker_2`))
  (bind _speaker_3 (`self.Speaker_3`))
  (bind _waterfallspeaker (`self.WaterfallSpeaker`))
  (bind _returnvalue (mod (`KismetSystemLibrary.GetGameTimeInSeconds`) (`self.SoundDuration`)))
  (`KismetSystemLibrary.PrintString` "Activating DRMusic")
  (`ActorComponent.Activate` _speaker_1 false)
  (`AudioComponent.Play` _speaker_1 _returnvalue)
  (`ActorComponent.Activate` _speaker_2 false)
  (`AudioComponent.Play` _speaker_2 _returnvalue)
  (`ActorComponent.Activate` _speaker_3 false)
  (`AudioComponent.Play` _speaker_3 _returnvalue)
  (`ActorComponent.Activate` _waterfallspeaker false)
  (`AudioComponent.Play` _waterfallspeaker 0.0)
  (set `self.bIsPlaying` true))

(fn `Deactivate_DRMusic`
  (`KismetSystemLibrary.PrintString` "Deactivating DRMusic")
  (`ActorComponent.Deactivate` (`self.Speaker_1`))
  (`ActorComponent.Deactivate` (`self.Speaker_2`))
  (`ActorComponent.Deactivate` (`self.Speaker_3`))
  (`ActorComponent.Deactivate` (`self.WaterfallSpeaker`))
  (set `self.bIsPlaying` false))

(fn `Load_DRMusic`)

(fn `Save_DRMusic`)

(fn `UserConstructionScript`)